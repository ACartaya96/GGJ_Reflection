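; CharacterSwitch is a trigger-box Blueprint that marks where character switching is allowed.
; On begin overlap, an actor tagged Ezekiel that casts to GGJ_CharacterController_BP gets CanChange set and debug text printed.
; The Ashton tag branch does nothing when true and wires back to the Ezekiel check when false, so actors with neither tag loop endlessly.
; End overlap clears CanChange on any such character, regardless of tag.
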(event `self.Box.OnComponentBeginOverlap`
  (params (OverlappedComponent :type "PrimitiveComponent Object Reference") (OtherActor :type "Actor Object Reference") (OtherComp :type "PrimitiveComponent Object Reference") (OtherBodyIndex :type Integer) (bFromSweep :type Boolean) (SweepResult :type "HitResult Structure (by ref)"))
  (if (`self.ActorHasTag` OtherActor "Ezekiel") :!label _label
    (bind _asggj_character_controller_bp (cast `/Game/Blueprints/GGJ_CharacterController_BP` OtherActor)
      (:`then`
        (bind _output_get (set `/Game/Blueprints/GGJ_CharacterController_BP.CanChange` true _asggj_character_controller_bp))
        (`KismetSystemLibrary.PrintString` "Ezikiel you can switch")
        (`KismetSystemLibrary.PrintString` (`KismetStringLibrary.Conv_BoolToString` _output_get)))
      (:`CastFailed`
        (if (not (`self.ActorHasTag` OtherActor "Ashton")) :!label _label_2
          (goto _label))))
    (else
      (goto _label_2))))

(event `self.Box.OnComponentEndOverlap`
  (params (OverlappedComponent :type "PrimitiveComponent Object Reference") (OtherActor :type "Actor Object Reference") (OtherComp :type "PrimitiveComponent Object Reference") (OtherBodyIndex :type Integer))
  (bind _asggj_character_controller_bp (cast `/Game/Blueprints/GGJ_CharacterController_BP` OtherActor))
  (set `/Game/Blueprints/GGJ_CharacterController_BP.CanChange` false _asggj_character_controller_bp))

(fn `UserConstructionScript`
  (`parent.UserConstructionScript`))
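; Movable mirror actor that swaps player control between the 2D and regular GGJ characters and can toggle physics on its mesh.
; DoInteraction checks the instigator's class, finds the other character type in the level and has player controller 0 possess it.
; X and Y axis collision overlaps switch physics simulation by "Ezekiel" tag.
; Only the Y begin-overlap tests the overlapping actor; the other three test the mirror's own tag.
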(event `self.DoInteraction`
  (params (Instigator :type "Actor Object Reference"))
  (bind _returnvalue (`GameplayStatics.GetObjectClass` Instigator))
  (bind _returnvalue_2 (`GameplayStatics.GetPlayerController` 0))
  (if (`KismetMathLibrary.ClassIsChildOf` _returnvalue "/Script/GGJ_Reflection.GGJ_2DCharacterController")
    (bind _returnvalue_3 (`GameplayStatics.GetActorOfClass` "/Script/GGJ_Reflection.GGJ_CharacterController"))
    (`/Engine/EditorBlueprintResources/StandardMacros.IsValid` _returnvalue_3
      (:`Is Valid`
        (`Controller.Possess` _returnvalue_2 _returnvalue_3)))
    (elif (`KismetMathLibrary.ClassIsChildOf` _returnvalue "/Script/GGJ_Reflection.GGJ_CharacterController")
      (bind _returnvalue_4 (`GameplayStatics.GetActorOfClass` "/Script/GGJ_Reflection.GGJ_2DCharacterController"))
      (`/Engine/EditorBlueprintResources/StandardMacros.IsValid` _returnvalue_4
        (:`Is Valid`
          (`Controller.Possess` _returnvalue_2 _returnvalue_4))))))

(event `self.YAxisCollision.OnComponentBeginOverlap`
  (params (OverlappedComponent :type "PrimitiveComponent Object Reference") (OtherActor :type "Actor Object Reference") (OtherComp :type "PrimitiveComponent Object Reference") (OtherBodyIndex :type Integer) (bFromSweep :type Boolean) (SweepResult :type "HitResult Structure (by ref)"))
  (if (`self.ActorHasTag` OtherActor "Ezekiel")
    (`PrimitiveComponent.SetSimulatePhysics` (`self.StaticMesh`) true)))

(event `self.XAxisCollision.OnComponentBeginOverlap`
  (params (OverlappedComponent :type "PrimitiveComponent Object Reference") (OtherActor :type "Actor Object Reference") (OtherComp :type "PrimitiveComponent Object Reference") (OtherBodyIndex :type Integer) (bFromSweep :type Boolean) (SweepResult :type "HitResult Structure (by ref)"))
  (if (`self.ActorHasTag` "Ezekiel")
    (`PrimitiveComponent.SetSimulatePhysics` (`self.StaticMesh`) true)))

(event `self.YAxisCollision.OnComponentEndOverlap`
  (params (OverlappedComponent :type "PrimitiveComponent Object Reference") (OtherActor :type "Actor Object Reference") (OtherComp :type "PrimitiveComponent Object Reference") (OtherBodyIndex :type Integer))
  (if (`self.ActorHasTag` "Ezekiel")
    (`PrimitiveComponent.SetSimulatePhysics` (`self.StaticMesh`) false)))

(event `self.XAxisCollision.OnComponentEndOverlap`
  (params (OverlappedComponent :type "PrimitiveComponent Object Reference") (OtherActor :type "Actor Object Reference") (OtherComp :type "PrimitiveComponent Object Reference") (OtherBodyIndex :type Integer))
  (if (`self.ActorHasTag` "Ezekiel")
    (`PrimitiveComponent.SetSimulatePhysics` (`self.StaticMesh`) false)))

(fn `UserConstructionScript`
  (`parent.UserConstructionScript`))